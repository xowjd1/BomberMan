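; BP_NetPlayerController is a player controller that connects chat input to the lobby HUD chat widget.
; The chat input action forwards an Enter key press to BPCTSComponent.
; Functions focus the chat input box and push username and message pairs into the widget when the HUD is valid.
; The all-players broadcast function is empty, with its per-controller update loop left disconnected.
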(event Input|EnhancedActionEvents|EnhancedInputActionIA_Chat
  (params (ActionValue :type Boolean) (ElapsedSeconds :type Float%20%28double-precision%29) (TriggeredSeconds :type Float%20%28double-precision%29) (InputAction :type Input%20Action%20Object%20Reference :default "/Game/Bluprints/enhancedInput/IA_Chat.IA_Chat"))
  (:Started
    (Default|KeyFunction (Variables|Default|GetBP_CTSComponent) "Enter")))

(fn ConstructionScript)

(fn FocusChat
  (bind _wb_lobbyhud (Variables|Default|GetWB_LobbyHUD)
    (:then
      (Class|Widget|SetUserFocus (Variables|/Game/TJ/Blueprints/WB_LobbyChat.WB_LobbyChat_C|GetChatMessage_InputBox (Variables|/Game/TJ/Blueprints/WB_LobbyHUD.WB_LobbyHUD_C|GetWB_LobbyChat _wb_lobbyhud)) self))
    (:else)))

(fn UpdateChatWidget
  (params (Username :type Text) (ChatMessage :type Text))
  (bind _wb_lobbyhud (Variables|Default|GetWB_LobbyHUD)
    (:then
      (Default|UpdateChat (Variables|/Game/TJ/Blueprints/WB_LobbyHUD.WB_LobbyHUD_C|GetWB_LobbyChat _wb_lobbyhud) Username ChatMessage))
    (:else)))

(fn UpdateChatforAllConnectedPlayers
  (params (ChatMessage :type Text)))